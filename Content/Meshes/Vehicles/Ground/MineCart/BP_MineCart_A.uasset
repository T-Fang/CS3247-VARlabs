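; BP_MineCart_A is a mine cart actor that lights up and shows a temporary text prompt when something enters its trigger box.
; On box overlap it turns on a spot and point light, then after a short delay shows shadowed text for a few seconds before hiding it.
; Ending the overlap hides the lights and text immediately, but pending delays are not cancelled and no overlapping-actor filter is applied.
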(event OnComponentBeginOverlap(Box)
  (params (OtherActor :type Actor%20Object%20Reference) (OtherComp :type Primitive%20Component%20Object%20Reference) (OtherBodyIndex :type Integer) (bFromSweep :type Boolean) (SweepResult :type Hit%20Result%20Structure%20%28by%20ref%29))
  (bind _textrender (Variables|Default|GetTextRender))
  ;[1 1 1] Jump In
  (Rendering|SetVisibility (Variables|Default|GetMinecart_SpotLight) true false)
  (Utilities|FlowControl|Delay 1.0)
  (Rendering|SetVisibility _textrender true false)
  (Utilities|FlowControl|Delay 3.0)
  (Rendering|SetVisibility _textrender false false))

(event OnComponentEndOverlap(Box)
  (params (OtherActor :type Actor%20Object%20Reference) (OtherComp :type Primitive%20Component%20Object%20Reference) (OtherBodyIndex :type Integer))
  ;[1 1 1] Jump Out
  (Rendering|SetVisibility (Variables|Default|GetMinecart_PointLight) false false))

(event EventBeginPlay)

(event EventActorBeginOverlap
  (params (OtherActor :type Actor%20Object%20Reference)))

(event EventTick
  (params (DeltaSeconds :type Float%20%28single-precision%29)))

(fn ConstructionScript)