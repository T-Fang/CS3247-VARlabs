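; BP_Chest_A is a chest prop that can open when a pawn comes near, controlled by the OpenWhenNear flag.
; Sphere overlap begin plays a timeline that rolls the lid open and turns on a point light.
; Overlap end reverses a second timeline to close the lid, leaving the light on.
; The construction script resets the lid to closed when the flag is set.
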(event OnComponentBeginOverlap(Sphere)
  (params (OtherActor :type Actor%20Object%20Reference) (OtherComp :type Primitive%20Component%20Object%20Reference) (OtherBodyIndex :type Integer) (bFromSweep :type Boolean) (SweepResult :type Hit%20Result%20Structure%20%28by%20ref%29))
  (if (Variables|Default|GetOpenWhenNear)
    (Utilities|Casting|CastToPawn OtherActor)
    (bind _curve_linear (Timeline|Open PlayFromStart)
      (:Update
        (Transformation|SetRelativeRotation (Variables|Default|GetChestLid) (Math|Rotator|MakeRotator (* _curve_linear -65.0) 0.0 0.0) false false)
        (Rendering|SetVisibility (Variables|Default|GetPointLight) true false)))))

(event OnComponentEndOverlap(Sphere)
  (params (OtherActor :type Actor%20Object%20Reference) (OtherComp :type Primitive%20Component%20Object%20Reference) (OtherBodyIndex :type Integer))
  (if (Variables|Default|GetOpenWhenNear)
    (Utilities|Casting|CastToPawn OtherActor)
    (bind _curve_linear (Timeline|Open2 ReverseFromEnd)
      (:Update
        (Transformation|SetRelativeRotation (Variables|Default|GetChestLid) (Math|Rotator|MakeRotator (* _curve_linear -65.0) 0.0 0.0) false false)))))

(event EventBeginPlay)

(event EventActorBeginOverlap
  (params (OtherActor :type Actor%20Object%20Reference)))

(event EventTick
  (params (DeltaSeconds :type Float%20%28single-precision%29)))

(fn ConstructionScript
  (if (Variables|Default|GetOpenWhenNear)
    (Transformation|SetRelativeRotation (Variables|Default|GetChestLid) "0.0,0.0,0.000000" false false)))