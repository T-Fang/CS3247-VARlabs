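; BP_Target_PopUp is a pop-up target actor that rises from its placed position and can be destroyed through interaction.
; After a random delay from BeginPlay, the UpAndDown timeline starts, and its curve drives a vertical offset from the stored origin.
; Interact spawns an emitter at the target's location, destroys the actor and returns a fixed integer to the caller.
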(event EventBeginPlay
  (Variables|Default|SetOrigin (Transformation|GetActorLocation))
  (Utilities|FlowControl|Delay (Math|Random|RandomFloatinRange 2.0 8.0))
  (bind _curve_mycurve (Timeline|UpAndDown PlayFromStart)
    (:Update
      (Transformation|SetActorLocation (+ (* "0, 0,20.000000" _curve_mycurve) (Variables|Default|GetOrigin)) false false))))

(fn ConstructionScript)

(fn Interact
  (Effects|SpawnEmitteratLocation 0 (Transformation|GetActorLocation) "0.000000, 0, 0")
  (Actor|DestroyActor)
  (return 5))