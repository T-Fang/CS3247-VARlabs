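; VR player for a two-stage Whack-A-Mole game, aimed by line traces along the camera's forward vector.
; Tick moves a billboard reticle to the gaze point and positions the hammer beside any hittable target.
; Act sends an interface hit message to the gazed target and increments Score, which drives GameStatus.
; Score thresholds swap the arcade moles and holes for the initially hidden BP_Holes stage, then stop that stage.
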(event EventTick
  (params (DeltaSeconds :type Float%20%28single-precision%29))
  (bind (_location _forward_vector) (CallFunction|GetPlayerVRCameraProperties))
  (bind (_outhit _returnvalue) (Collision|LineTraceByChannel _location (+ _location (* _forward_vector 1e+04)) "TraceTypeQuery1" false 0 "None"))
  (if _returnvalue
    (Transformation|SetWorldLocation (Variables|Default|GetMaterialBillboard) (.Location (Collision|BreakHitResult _outhit)) false false)
    (bind _ishittable (Class|BPIHittable|IsHittable(Message) (.HitActor (Collision|BreakHitResult _outhit))))
    (if _ishittable
      (bind _returnvalue_2 (Actor|GetActorOfClass "/Game/Lessons/Lesson3/miniProject3/BP_Hammer_Origin.BP_Hammer_Origin_C"))
      (Transformation|SetWorldLocation (Variables|/Game/Lessons/Lesson3/miniProject3/BP_Hammer_Origin.BP_Hammer_Origin_C|GetDefaultSceneRoot1 _returnvalue_2) (+ (.Location (Collision|BreakHitResult _outhit)) "0,25.000000,15.000000") false false))
    (else
      (Transformation|SetWorldLocation (Variables|Default|GetMaterialBillboard) (+ _location (* _forward_vector 1e+04)) false false))))

(event EventBeginPlay
  (bind _outactors (Actor|GetAllActorsOfClass "/Game/Lessons/Lesson3/miniProject3/BP_Holes.BP_Holes_C"))
  (for _array_element _outactors
    (Rendering|SetVisibility (Variables|/Game/Lessons/Lesson3/miniProject3/BP_Holes.BP_Holes_C|GetSharedRoot _array_element) false true)))

(fn ConstructionScript)

(fn Act
  (bind (_location _forward_vector) (CallFunction|GetPlayerVRCameraProperties))
  (bind (_outhit _returnvalue) (Collision|LineTraceByChannel _location (+ _location (* _forward_vector 1e+04)) "TraceTypeQuery1" false 0 "None"))
  (if _returnvalue
    (bind _ishittable (Class|BPIHittable|IsHittable(Message) (.HitActor (Collision|BreakHitResult _outhit))))
    (if _ishittable
      ;[1 1 1] Note: even if the target is not a BPI Hittable, the nodes following this node will continue to execute, but we only want to add score when it is hittable. Hence, a "Is Hittable" branch is added before this node
      (Class|BPIHittable|Hit(Message) (.HitActor (Collision|BreakHitResult _outhit)))
      (bind _output_get (Variables|Default|SetScore (+ 1 (Variables|Default|GetScore))))
      (switch int (Variables|Default|GetGameStatus)
        (:0
          ;[1 1 1] First Game - Normal arcade machine Whack A Mole
          (if (> _output_get 4)
            (bind _outactors (Actor|GetAllActorsOfClass "/Game/Lessons/Lesson3/miniProject3/BP_Mole.BP_Mole_C"))
            (for _array_element _outactors
              (Default|StopPopping _array_element))
            (bind _outactors_2 (Actor|GetAllActorsOfClass "/Game/Lessons/Lesson3/miniProject3/BP_Hole.BP_Hole_C"))
            (for _array_element_2 _outactors_2
              (Actor|DestroyActor _array_element_2))
            (Variables|Default|SetGameStatus 1)
            (bind _outactors_3 (Actor|GetAllActorsOfClass "/Game/Lessons/Lesson3/miniProject3/BP_Holes.BP_Holes_C"))
            (for _array_element_3 _outactors_3
              (Rendering|SetVisibility (Variables|/Game/Lessons/Lesson3/miniProject3/BP_Holes.BP_Holes_C|GetSharedRoot _array_element_3) true true))))
        (:1
          ;[1 1 1] First Game - Now the Mole is the arcade machine itself
          (if (> _output_get 9)
            (bind _outactors_4 (Actor|GetAllActorsOfClass "/Game/Lessons/Lesson3/miniProject3/BP_Holes.BP_Holes_C"))
            (for _array_element_4 _outactors_4
              (Default|StopPopping _array_element_4)
              (Variables|Default|SetGameStatus 2))))))))

(fn IsFacingHittable
  (bind (_location _forward_vector) (CallFunction|GetPlayerVRCameraProperties))
  (bind (_outhit _returnvalue) (Collision|LineTraceByChannel _location (+ _location (* _forward_vector 1e+04)) "TraceTypeQuery1" false 0 "None"))
  (if _returnvalue
    (bind _ishittable (Class|BPIHittable|IsHittable(Message) (.HitActor (Collision|BreakHitResult _outhit))))
    (return _ishittable)))