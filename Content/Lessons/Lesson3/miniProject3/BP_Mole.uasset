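; BP_Mole is a whack-a-mole style target actor that repeatedly pops up from its starting position at random intervals.
; After a random initial delay, the PopUp timeline offsets it vertically along a curve, then replays after another random wait on each finish.
; Hit spawns a small neon explosion and resets the timeline time, while StopPopping destroys the actor.
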(event EventStopPopping
  (Actor|DestroyActor))

(event EventBeginPlay
  (Variables|Default|SetdefaultPosition (Transformation|GetActorLocation))
  (Utilities|FlowControl|Delay (Math|Random|RandomFloatinRange 0.0 1e+01))
  (bind _curve_mole (Timeline|PopUp PlayFromStart)
    (:Update
      (Transformation|SetActorLocation (+ (* "0, 0,105.000000" _curve_mole) (Variables|Default|GetdefaultPosition)) false false))
    (:Finished
      (Utilities|FlowControl|Delay (Math|Random|RandomFloatinRange 4.0 1e+01))
      (Timeline|PopUp PlayFromStart))))

(event EventHit
  (Effects|SpawnEmitteratLocation "/Game/Effects/Particles/Explosion/P_NeonExplosion_Tiny.P_NeonExplosion_Tiny" (Transformation|GetActorLocation))
  (bind _curve_mole (Timeline|PopUp SetNewTime)
    (:Update
      (Transformation|SetActorLocation (+ (* "0, 0,105.000000" _curve_mole) (Variables|Default|GetdefaultPosition)) false false))
    (:Finished
      (Utilities|FlowControl|Delay (Math|Random|RandomFloatinRange 4.0 1e+01))
      (Timeline|PopUp PlayFromStart))))

(fn ConstructionScript)