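; BP_Target_ColorChange is a target actor that randomly changes color and value, including a negative one, while in play.
; From BeginPlay, ChangeType picks blue, gray or yellow, sets the matching material and Value, then calls itself again after a random delay of a few seconds.
; Interact spawns an emitter slightly offset from the target, destroys the actor and returns the current Value to the caller.
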(event Custom|ChangeType
  (switch int (Math|Random|RandomIntegerinRange 0 2)
    (:0
      (Rendering|Material|SetMaterial (Variables|Default|GetTarget) 0 "/Game/Materials/Props/Combat/Targets/MI_Targets_Blue.MI_Targets_Blue")
      (Variables|Default|SetValue 10))
    (:1
      (Rendering|Material|SetMaterial (Variables|Default|GetTarget) 0 "/Game/Materials/Props/Combat/Targets/MI_Targets_Gray.MI_Targets_Gray")
      (Variables|Default|SetValue 5))
    (:2
      (Rendering|Material|SetMaterial (Variables|Default|GetTarget) 0 "/Game/Materials/Props/Combat/Targets/MI_Targets_Yellow.MI_Targets_Yellow")
      (Variables|Default|SetValue -5)))
  (Utilities|FlowControl|Delay (Math|Random|RandomFloatinRange 2.0 6.0))
  (CallFunction|ChangeType))

(event EventBeginPlay
  (CallFunction|ChangeType))

(event Collision|EventActorBeginOverlap
  (params (OtherActor :type Actor%20Object%20Reference)))

(event EventTick
  (params (DeltaSeconds :type Float%20%28single-precision%29)))

(fn ConstructionScript)

(fn Interact
  (Effects|SpawnEmitteratLocation 0 (+ (Transformation|GetActorLocation) "-25.000000, 0, 0"))
  (Actor|DestroyActor)
  (return (Variables|Default|GetValue)))