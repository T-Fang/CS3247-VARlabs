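; Spaceship actor that flies in a straight line toward the world origin and disappears when it gets close.
; On BeginPlay it picks a random speed and sets its direction to the negated, normalized spawn location.
; Each Tick it offsets itself along that direction without sweep or delta-time scaling, so movement is frame-rate dependent.
; It destroys itself once it is within a fixed radius of the origin.
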(event EventBeginPlay
  (Variables|Default|SetSpeed (Math|Random|RandomFloatinRange 4e+01 6e+01))
  (Variables|Default|Setdirection (Math|Vector|NegateVector (Math|Vector|Normalize (Transformation|GetActorLocation)))))

(event Collision|EventActorBeginOverlap
  (params (OtherActor :type Actor%20Object%20Reference)))

(event EventTick
  (params (DeltaSeconds :type Float%20%28single-precision%29))
  (if (<= (Math|Vector|VectorLength (Transformation|GetActorLocation)) 1e+03)
    (Actor|DestroyActor)
    (else
      (Transformation|AddActorWorldOffset (* (Variables|Default|Getdirection) (Variables|Default|GetSpeed))))))

(fn ConstructionScript)