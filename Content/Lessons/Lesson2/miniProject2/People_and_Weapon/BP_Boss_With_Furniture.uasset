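; BP_Boss_With_Furniture is a lesson mini-project actor that shows a boss's threatening dialogue through a TextRender component.
; On BeginPlay it sets a first line scolding disobedience, then after a short Delay replaces it with a second threat.
; Overlap and Tick events are disabled, the construction script is empty, and a leftover location calculation is unused.
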(event EventBeginPlay
  (Rendering|Components|TextRender|SetText (Variables|Default|GetTextRender) (Utilities|Text|ToText(String) (Utilities|String|MakeLiteralString "This is what you get when <br> you disobeyed my order")))
  (Utilities|FlowControl|Delay 3.0)
  (Rendering|Components|TextRender|SetText (Variables|Default|GetTextRender) (Utilities|Text|ToText(String) (Utilities|String|MakeLiteralString "I could kill you with a gun<br>But that would be too easy"))))

(event Collision|EventActorBeginOverlap
  (params (OtherActor :type Actor%20Object%20Reference)))

(event EventTick
  (params (DeltaSeconds :type Float%20%28single-precision%29)))

(fn ConstructionScript)