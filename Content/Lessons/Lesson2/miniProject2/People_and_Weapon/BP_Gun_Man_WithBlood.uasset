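; BP_Gun_Man_WithBlood is a lesson mini-project actor that plays a scripted gunfire death as soon as play begins.
; BeginPlay plays a machine gun sound at the skeletal mesh, then waits briefly.
; It then reveals two blood stains, rolls the mesh 90 degrees to topple it and plays a death scream.
; The sequence is purely timed, with no overlap, damage or tick logic.
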(event EventBeginPlay
  (Audio|PlaySoundatLocation "/Game/Audio/Tian_Fang/Fight/Machine_Gun.Machine_Gun" (Transformation|GetWorldLocation (Variables|Default|GetSkeletalMesh)) "0, 0, 0" 1.0 1.0 0.0 0 0 0)
  (Utilities|FlowControl|Delay 1.2)
  (Rendering|SetVisibility (Variables|Default|GetBloodStain) true false)
  (Rendering|SetVisibility (Variables|Default|GetBloodStain2) true false)
  (Transformation|AddLocalRotation (Variables|Default|GetSkeletalMesh) (Math|Rotator|MakeRotator 9e+01 0.0 0.0) false false)
  (Audio|PlaySoundatLocation "/Game/Audio/Tian_Fang/Fight/Man_Death_Scream2.Man_Death_Scream2" (Transformation|GetWorldLocation (Variables|Default|GetSkeletalMesh)) "0, 0, 0" 1.0 1.0 0.0 0 0 0))

(event Collision|EventActorBeginOverlap
  (params (OtherActor :type Actor%20Object%20Reference)))

(event EventTick
  (params (DeltaSeconds :type Float%20%28single-precision%29)))

(fn ConstructionScript)