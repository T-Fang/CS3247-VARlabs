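; BP_Axe_2 is a thrown axe that launches itself toward the player's head, using BP_Old_Chair's location plus an upward bias.
; After a fixed delay plus random jitter on BeginPlay, it locks in direction, picks a random speed and plays a throw sound.
; Tick spins and sweeps it forward without delta-time scaling until it overlaps anything other than another axe.
; MoveAxe duplicates that motion with fixed values but is not called here.
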(event OnComponentBeginOverlap(Axe)
  (params (OverlappedComponent :type Primitive%20Component%20Object%20Reference) (OtherActor :type Actor%20Object%20Reference) (OtherComp :type Primitive%20Component%20Object%20Reference) (OtherBodyIndex :type Integer) (bFromSweep :type Boolean) (SweepResult :type Hit%20Result%20Structure%20%28by%20ref%29))
  (if (not (== (Utilities|GetClass OtherActor) "BP_Axe_2_C"))
    (Variables|Default|SetisAxeMoving false)))

(event EventBeginPlay
  (Utilities|FlowControl|Delay 6.0)
  (Utilities|FlowControl|Delay (Math|Random|RandomFloatinRange 0.0 1.0))
  (bind _returnvalue (Actor|GetActorOfClass "/Game/Lessons/Lesson2/miniProject2/House/Interior/BP_Old_Chair.BP_Old_Chair_C"))
  (Variables|Default|Setdirection (+ (Math|Vector|GetUnitDirection(Vector) (Transformation|GetActorLocation) (Transformation|GetActorLocation _returnvalue)) "0.000000, 0,0.300000"))
  (Variables|Default|SetisAxeMoving true)
  (Variables|Default|SetSpeed (Math|Random|RandomFloatinRange 2e+01 4e+01))
  (Audio|PlaySoundatLocation "/Game/Audio/Tian_Fang/Fight/Throw_Weapon.Throw_Weapon" (Transformation|GetWorldLocation (Variables|Default|GetAxe)) "0, 0, 0" 1.0 1.0 0.0 0 0 0))

(event Collision|EventActorBeginOverlap
  (params (OtherActor :type Actor%20Object%20Reference)))

(event EventTick
  (params (DeltaSeconds :type Float%20%28single-precision%29))
  (if (Variables|Default|GetisAxeMoving)
    (Transformation|AddActorLocalRotation "0.000000,-60.000000,0.000000" false false)
    (Transformation|AddActorWorldOffset (* (Variables|Default|Getdirection) (Variables|Default|GetSpeed)) true)))

(fn ConstructionScript)

(fn MoveAxe
  (if (Variables|Default|GetisAxeMoving)
    (Transformation|AddActorLocalRotation "0.000000,-22.000000,0.000000" false false)
    (Transformation|AddActorWorldOffset (* (Variables|Default|Getdirection) 2e+01) true)))