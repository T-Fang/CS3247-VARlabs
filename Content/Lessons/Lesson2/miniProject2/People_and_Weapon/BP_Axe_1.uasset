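; BP_Axe_1 is a thrown axe actor that spins as it flies toward the gun man character.
; BeginPlay caches a one-time direction to BP_Gun_Man_WithBlood, so the axe does not home.
; While IsAxeMoving is true, Tick rotates it and applies a swept world offset at a fixed per-frame step until the Axe component's overlap clears the flag.
; A MoveAxe function holds near-identical movement logic but is not called within this Blueprint.
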(event OnComponentBeginOverlap(Axe)
  (params (OverlappedComponent :type Primitive%20Component%20Object%20Reference) (OtherActor :type Actor%20Object%20Reference) (OtherComp :type Primitive%20Component%20Object%20Reference) (OtherBodyIndex :type Integer) (bFromSweep :type Boolean) (SweepResult :type Hit%20Result%20Structure%20%28by%20ref%29))
  (Variables|Default|SetisAxeMoving false))

(event EventBeginPlay
  (bind _returnvalue (Actor|GetActorOfClass "/Game/Lessons/Lesson2/miniProject2/People_and_Weapon/BP_Gun_Man_WithBlood.BP_Gun_Man_WithBlood_C"))
  (Variables|Default|Setdirection (Math|Vector|GetUnitDirection(Vector) (Transformation|GetActorLocation) (Transformation|GetActorLocation _returnvalue))))

(event Collision|EventActorBeginOverlap
  (params (OtherActor :type Actor%20Object%20Reference)))

(event EventTick
  (params (DeltaSeconds :type Float%20%28single-precision%29))
  (if (Variables|Default|GetisAxeMoving)
    (Transformation|AddActorLocalRotation "0.000000,-25.000000,0.000000" false false)
    (Transformation|AddActorWorldOffset (* (Variables|Default|Getdirection) 2e+01) true)))

(fn ConstructionScript)

(fn MoveAxe
  (if (Variables|Default|GetisAxeMoving)
    (Transformation|AddActorLocalRotation "0.000000,-22.000000,0.000000" false false)
    (Transformation|AddActorWorldOffset (* (Variables|Default|Getdirection) 2e+01) true)))