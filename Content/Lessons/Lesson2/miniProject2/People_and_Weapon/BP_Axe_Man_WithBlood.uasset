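; Axe man character actor that plays a scripted, timed attack-and-death sequence as soon as play begins.
; BeginPlay plays machine gun and attack sounds at the skeletal mesh, then waits briefly.
; It then reveals two blood stains, rolls the mesh onto its side and plays a death scream.
; The overlap and tick events are disabled and the construction script is empty.
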(event EventBeginPlay
  (bind _skeletalmesh (Variables|Default|GetSkeletalMesh))
  (bind _returnvalue (Transformation|GetWorldLocation _skeletalmesh))
  (Audio|PlaySoundatLocation "/Game/Audio/Tian_Fang/Fight/Machine_Gun.Machine_Gun" _returnvalue "0, 0, 0" 1.0 1.0 0.0 0 0 0)
  (Audio|PlaySoundatLocation "/Game/Audio/Tian_Fang/Fight/Man_Attack.Man_Attack" _returnvalue "0, 0, 0" 1.0 1.0 0.0 0 0 0)
  (Utilities|FlowControl|Delay 1.2)
  (Rendering|SetVisibility (Variables|Default|GetBloodStain1) true false)
  (Rendering|SetVisibility (Variables|Default|GetBloodStain2) true false)
  (Transformation|AddLocalRotation (Variables|Default|GetSkeletalMesh) (Math|Rotator|MakeRotator 9e+01 0.0 0.0) false false)
  (Audio|PlaySoundatLocation "/Game/Audio/Tian_Fang/Fight/Man_Death_Scream1.Man_Death_Scream1" (Transformation|GetWorldLocation (Variables|Default|GetSkeletalMesh)) "0, 0, 0" 1.0 1.0 0.0 0 0 0))

(event Collision|EventActorBeginOverlap
  (params (OtherActor :type Actor%20Object%20Reference)))

(event EventTick
  (params (DeltaSeconds :type Float%20%28single-precision%29)))

(fn ConstructionScript)