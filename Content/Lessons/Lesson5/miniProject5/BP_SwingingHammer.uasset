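; Swinging hammer obstacle that knocks a FallGuysPlayer away on contact.
; After random and configurable start delays, a timeline drives the hammer's pitch, playing forward once then restarting in reverse on each finish, with a delayed swing sound each pass.
; Box overlap applies zero damage and launches the player along the Arrow's forward vector scaled by LaunchSpeed.
; A second timeline loop is never run, and Damage is unused.
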(event OnComponentBeginOverlap(Box)
  (params (OverlappedComponent :type Primitive%20Component%20Object%20Reference) (OtherActor :type Actor%20Object%20Reference) (OtherComp :type Primitive%20Component%20Object%20Reference) (OtherBodyIndex :type Integer) (bFromSweep :type Boolean) (SweepResult :type Hit%20Result%20Structure%20%28by%20ref%29))
  (bind _asfall_guys_player (Utilities|Casting|CastToFallGuysPlayer OtherActor))
  (Default|ApplyDamage _asfall_guys_player 0.0)
  (Character|LaunchCharacter _asfall_guys_player (* (Math|Vector|GetForwardVector (Variables|Components|GetArrow)) (Variables|Default|GetlaunchSpeed)) false false))

(event EventBeginPlay
  (bind _returnvalue (Transformation|GetActorLocation))
  (Utilities|FlowControl|Delay (Math|Random|RandomFloatinRange 0.0 1.0))
  (Utilities|FlowControl|Delay (Variables|Default|GetDelay))
  (Utilities|FlowControl|Sequence
    (:then_0
      (Utilities|FlowControl|Delay 0.5)
      (Audio|PlaySoundatLocation "/Game/Audio/Tian_Fang/Foley/Swing.Swing" _returnvalue "0, 0, 0" 0.5 1.0 0.0 0 0 0))
    (:then_1
      (bind _swing (Timeline|Timeline_0 PlayFromStart)
        (:Update
          (Transformation|SetRelativeRotation (Variables|Components|GetHammer) (Math|Rotator|MakeRotator 1.8e+02 _swing 0.0) false false))
        (:Finished
          (Utilities|FlowControl|Sequence
            (:then_0
              (Utilities|FlowControl|Delay 0.5)
              (Audio|PlaySoundatLocation "/Game/Audio/Tian_Fang/Foley/Swing.Swing" _returnvalue "0, 0, 0" 0.5 1.0 0.0 0 0 0))
            (:then_1
              (Timeline|Timeline_0 ReverseFromEnd))))))))

(fn ConstructionScript)