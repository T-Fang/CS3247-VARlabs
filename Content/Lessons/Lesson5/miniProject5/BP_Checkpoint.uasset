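; BP_Checkpoint is a checkpoint button that saves its location, raised slightly, to the FirstPersonGameMode when its box is overlapped.
; The first FallGuysPlayer overlap also plays a timeline that moves the button, then marks it pressed, restores the player's health and fires sounds and a particle burst.
; Once pressed, later overlaps by any actor only update the saved checkpoint.
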(event OnComponentBeginOverlap(Box)
  (params (OverlappedComponent :type Primitive%20Component%20Object%20Reference) (OtherActor :type Actor%20Object%20Reference) (OtherComp :type Primitive%20Component%20Object%20Reference) (OtherBodyIndex :type Integer) (bFromSweep :type Boolean) (SweepResult :type Hit%20Result%20Structure%20%28by%20ref%29))
  (bind _returnvalue (Transformation|GetActorLocation))
  (if (Variables|Default|GetPressed)
    (bind _asfirst_person_game_mode (Utilities|Casting|CastToFirstPersonGameMode (Game|GetGameMode)))
    (Variables|/Game/Lessons/Lesson4/FirstPerson/FirstPersonGameMode.FirstPersonGameMode_C|SetCheckPoint _asfirst_person_game_mode (+ (Transformation|GetActorLocation) "0, 0,100.000000"))
    (else
      (bind _asfall_guys_player (Utilities|Casting|CastToFallGuysPlayer OtherActor))
      (bind _asfirst_person_game_mode_2 (Utilities|Casting|CastToFirstPersonGameMode (Game|GetGameMode)))
      (Variables|/Game/Lessons/Lesson4/FirstPerson/FirstPersonGameMode.FirstPersonGameMode_C|SetCheckPoint _asfirst_person_game_mode_2 (+ (Transformation|GetActorLocation) "0, 0,100.000000"))
      (bind _newtrack_0 (Timeline|Timeline_0 Play)
        (:Update
          (Transformation|SetRelativeLocation (Variables|Default|GetButton) (Math|Vector|MakeVector 0.0 0.0 (* _newtrack_0 0.1)) false false))
        (:Finished
          (Variables|Default|SetPressed true)
          (Variables|/Game/Lessons/Lesson5/miniProject5/FallGuysPlayer.FallGuysPlayer_C|SetCurrentHealth _asfall_guys_player (Variables|/Game/Lessons/Lesson5/miniProject5/FallGuysPlayer.FallGuysPlayer_C|GetMaxHealth _asfall_guys_player))
          (Audio|PlaySoundatLocation "/Game/Audio/Tian_Fang/Foley/Button_Pressed.Button_Pressed" _returnvalue "0, 0, 0" 1.0 1.0 0.0 0 0 0)
          (Effects|SpawnEmitteratLocation "/Game/Effects/Particles/Explosion/P_NeonExplosion.P_NeonExplosion" _returnvalue)
          (Audio|PlaySoundatLocation "/Game/Audio/Tian_Fang/Foley/Firework_Blast.Firework_Blast" _returnvalue "0, 0, 0" 1.0 1.0 0.0 0 0 0))))))

(event EventBeginPlay)

(event Collision|EventActorBeginOverlap
  (params (OtherActor :type Actor%20Object%20Reference)))

(event EventTick
  (params (DeltaSeconds :type Float%20%28single-precision%29)))

(fn ConstructionScript)