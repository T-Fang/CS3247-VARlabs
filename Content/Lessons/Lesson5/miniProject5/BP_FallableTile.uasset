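; BP_FallableTile is a tile actor that falls after something overlaps its trigger box.
; The overlap starts a configurable delay, then applies linear and angular damping and enables physics simulation on the static mesh.
; When destroyed, a respawnable tile spawns a replacement at the transform saved on BeginPlay, with physics off and its tuning variables copied over.
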(event OnComponentBeginOverlap(Box)
  (params (OverlappedComponent :type Primitive%20Component%20Object%20Reference) (OtherActor :type Actor%20Object%20Reference) (OtherComp :type Primitive%20Component%20Object%20Reference) (OtherBodyIndex :type Integer) (bFromSweep :type Boolean) (SweepResult :type Hit%20Result%20Structure%20%28by%20ref%29))
  (bind _staticmeshcomponent (Variables|Debug|GetStaticMeshComponent))
  (Utilities|FlowControl|Delay (Variables|Default|GetDelay))
  (Class|PrimitiveComponent|SetLinearDamping (Variables|Debug|GetStaticMeshComponent) (Variables|Default|GetLinearDamping))
  (Class|PrimitiveComponent|SetAngularDamping _staticmeshcomponent (Variables|Default|GetAngular%20Damping))
  (Physics|SetSimulatePhysics _staticmeshcomponent true))

(event EventDestroyed
  (if (Variables|Default|GetRespawnable)
    (bind _returnvalue (Game|SpawnActorfromClass "BP_FallableTile_C" (Variables|Default|GetStart%20Transform) "Undefined" self 0))
    (Physics|SetSimulatePhysics (Variables|/Script/Engine.StaticMeshActor|GetStaticMeshComponent _returnvalue) false)
    (Variables|BP_FallableTile_C|SetAngular%20Damping _returnvalue (Variables|Default|GetAngular%20Damping))
    (Variables|BP_FallableTile_C|SetDelay _returnvalue (Variables|Default|GetDelay))
    (Variables|BP_FallableTile_C|SetRespawnable _returnvalue (Variables|Default|GetRespawnable))
    (Variables|BP_FallableTile_C|SetLinearDamping _returnvalue (Variables|Default|GetLinearDamping))))

(event EventBeginPlay
  (Variables|Default|SetStart%20Transform (Transformation|GetActorTransform)))

(fn ConstructionScript)