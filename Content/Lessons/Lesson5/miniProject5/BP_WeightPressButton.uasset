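; Pressure button for a lesson mini-project that moves when something enters or leaves its trigger box, with no weight check.
; Begin and end overlap each stop the opposite timeline and play their own, setting the Button's relative Z from its Force track.
; Both overlaps play a sound, guarded by a shared flag and short delay against repeats.
; Either timeline prints "Button Pressed" on finishing, including the end-overlap one.
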(event OnComponentBeginOverlap(Box)
  (params (OverlappedComponent :type Primitive%20Component%20Object%20Reference) (OtherActor :type Actor%20Object%20Reference) (OtherComp :type Primitive%20Component%20Object%20Reference) (OtherBodyIndex :type Integer) (bFromSweep :type Boolean) (SweepResult :type Hit%20Result%20Structure%20%28by%20ref%29))
  (Utilities|FlowControl|Sequence
    (:then_0
      (bind _force (Timeline|Timeline_1 Stop)
        (:Update
          (Transformation|SetRelativeLocation (Variables|Default|GetButton) (Math|Vector|MakeVector 0.0 0.0 (Math|Float|Lerp _force 0.0 0.0)) false false))
        (:Finished
          (Development|PrintString "Button Pressed"))))
    (:then_1
      (if (not (Variables|Default|GetPlayingSound))
        (Variables|Default|SetPlayingSound true)
        (Audio|SpawnSoundatLocation 0 (Transformation|GetActorLocation) "0, 0, 0" 1.0 1.0 0.0 0 0)
        (Utilities|FlowControl|Delay 0.3)
        (Variables|Default|SetPlayingSound false)))
    (:then_2
      (bind _force_2 (Timeline|Timeline_0 Play)
        (:Update
          (Transformation|SetRelativeLocation (Variables|Default|GetButton) (Math|Vector|MakeVector 0.0 0.0 (Math|Float|Lerp _force_2 0.0 0.0)) false false))
        (:Finished
          (Development|PrintString "Button Pressed"))))))

(event OnComponentEndOverlap(Box)
  (params (OverlappedComponent :type Primitive%20Component%20Object%20Reference) (OtherActor :type Actor%20Object%20Reference) (OtherComp :type Primitive%20Component%20Object%20Reference) (OtherBodyIndex :type Integer))
  (Utilities|FlowControl|Sequence
    (:then_0
      (bind _force (Timeline|Timeline_0 Stop)
        (:Update
          (Transformation|SetRelativeLocation (Variables|Default|GetButton) (Math|Vector|MakeVector 0.0 0.0 (Math|Float|Lerp _force 0.0 0.0)) false false))
        (:Finished
          (Development|PrintString "Button Pressed"))))
    (:then_1
      (if (not (Variables|Default|GetPlayingSound))
        (Variables|Default|SetPlayingSound true)
        (Audio|SpawnSoundatLocation 0 (Transformation|GetActorLocation) "0, 0, 0" 1.0 1.0 0.0 0 0)
        (Utilities|FlowControl|Delay 0.3)
        (Variables|Default|SetPlayingSound false)))
    (:then_2
      (bind _force_2 (Timeline|Timeline_1 Play)
        (:Update
          (Transformation|SetRelativeLocation (Variables|Default|GetButton) (Math|Vector|MakeVector 0.0 0.0 (Math|Float|Lerp _force_2 0.0 0.0)) false false))
        (:Finished
          (Development|PrintString "Button Pressed"))))))

(fn ConstructionScript)