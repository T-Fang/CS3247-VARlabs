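; BP_Rocket is a lesson actor that launches as a physics-driven rocket when interacted with.
; PhysicsInteract calls FireRocket with no delay, and FireRocket can also take a delay before launch.
; Launch enables mesh physics simulation, the physics thruster and a particle system.
; After a fixed flight time, it spawns an asteroid explosion effect at the mesh location and destroys itself.
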(event Custom|Fire%20Rocket
  (params (Delay :type Float%20%28single-precision%29))
  (Utilities|FlowControl|Delay Delay)
  (Physics|SetSimulatePhysics (Variables|Default|GetStaticMesh) true)
  (Components|Activation|SetActive (Variables|Default|GetPhysicsThruster) true false)
  (Components|Activation|Activate (Variables|Default|GetTutorialParticleSystem) false)
  (Utilities|FlowControl|Delay 1e+01)
  (Effects|SpawnEmitteratLocation "/Game/Effects/Particles/Explosion/P_AsteroidExplosion.P_AsteroidExplosion" (Transformation|GetWorldLocation (Variables|Default|GetStaticMesh)) "0, 0, 0" "1.000000,1.000000,1.000000" false)
  (Actor|DestroyActor))

(event EventPhysicsInteract
  (CallFunction|FireRocket 0.0))

(fn ConstructionScript)