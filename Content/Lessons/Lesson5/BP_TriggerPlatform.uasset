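; BP_TriggerPlatform is a lesson trigger platform actor that gives color and sound feedback when something enters or leaves its box.
; On Box begin overlap, it sets the "Color" material parameter on two static meshes to green and plays a laser sound.
; On end overlap, it sets the same parameter to blue and plays a chime.
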(event OnComponentBeginOverlap(Box)
  (params (OverlappedComponent :type Primitive%20Component%20Object%20Reference) (OtherActor :type Actor%20Object%20Reference) (OtherComp :type Primitive%20Component%20Object%20Reference) (OtherBodyIndex :type Integer) (bFromSweep :type Boolean) (SweepResult :type Hit%20Result%20Structure%20%28by%20ref%29))
  (Rendering|Material|SetVectorParameterValueonMaterials (Variables|Default|GetStaticMesh1) "Color" (Math|Conversions|ToVector(LinearColor) "(R=0.000000,G=1.000000,B=0.000000,A=1.000000)"))
  (Audio|Components|Audio|Play (Variables|Default|GetSW_Laser_3) 0.0))

(event OnComponentEndOverlap(Box)
  (params (OverlappedComponent :type Primitive%20Component%20Object%20Reference) (OtherActor :type Actor%20Object%20Reference) (OtherComp :type Primitive%20Component%20Object%20Reference) (OtherBodyIndex :type Integer))
  (Rendering|Material|SetVectorParameterValueonMaterials (Variables|Default|GetStaticMesh1) "Color" (Math|Conversions|ToVector(LinearColor) "(R=0.000000,G=0.287324,B=1.000000,A=1.000000)"))
  (Audio|Components|Audio|Play (Variables|Default|GetSW_Chime_1) 0.0))

(event EventBeginPlay)

(event EventActorBeginOverlap
  (params (OtherActor :type Actor%20Object%20Reference)))

(event EventTick
  (params (DeltaSeconds :type Float%20%28single-precision%29)))

(fn ConstructionScript)